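; Pressure plate that toggles a referenced Piedra (stone) object when the third-person character or an AI_Sphere steps on or off it.
; Begin and end overlaps on the Collision component each call SwitchOnOff on PiedraRef, with no count of how many actors are on the plate.
; A timeline plays on entry and reverses on exit, lerping the Placa component's relative Z to sink and raise the plate.
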(event `self.Collision.OnComponentBeginOverlap`
  (params (OverlappedComponent :type "PrimitiveComponent Object Reference") (OtherActor :type "Actor Object Reference") (OtherComp :type "PrimitiveComponent Object Reference") (OtherBodyIndex :type Integer) (bFromSweep :type Boolean) (SweepResult :type "HitResult Structure (by ref)"))
  (cast `/Game/Bichitos/AI_Sphere` OtherActor
    (:`then`
      _)
    (:`CastFailed`
      (cast `/Game/ThirdPerson/Blueprints/BP_ThirdPersonCharacter` OtherActor)))
  (`/Game/Piedra_Up/BP_PiedraUp.SwitchOn/Off` (`self.PiedraRef`))
  (bind (_direction _newtrack_0) (`Timeline|Plate Timelien` :!label _label)
    (:`Update`
      (`SceneComponent.K2_SetRelativeLocation` (`self.Placa`) (`KismetMathLibrary.MakeVector` 0.0 0.0 (`KismetMathLibrary.Lerp` 4.5 1.0 _newtrack_0)) false false))))

(event `self.Collision.OnComponentEndOverlap`
  (params (OverlappedComponent :type "PrimitiveComponent Object Reference") (OtherActor :type "Actor Object Reference") (OtherComp :type "PrimitiveComponent Object Reference") (OtherBodyIndex :type Integer))
  (cast `/Game/Bichitos/AI_Sphere` OtherActor
    (:`then`
      _)
    (:`CastFailed`
      (cast `/Game/ThirdPerson/Blueprints/BP_ThirdPersonCharacter` OtherActor)))
  (`/Game/Piedra_Up/BP_PiedraUp.SwitchOn/Off` (`self.PiedraRef`))
  (goto _label :!via `Reverse`))

(fn `UserConstructionScript`)